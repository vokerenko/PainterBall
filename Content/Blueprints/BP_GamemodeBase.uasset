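; Base game mode that tracks level objective totals and presents the win screen.
; On BeginPlay it counts all Target and PurifierTarget actors in the level and stores both totals.
; The OnWin event adds the WB_Win widget to the viewport for the first player and switches input to UI only.
; No win condition is evaluated here, and nothing in this graph calls OnWin.
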(event EventBeginPlay
  (bind _outactors (Actor|GetAllActorsOfClass "/Script/PainterBall.Target"))
  (Variables|Default|SetTotalTargetsCount (Utilities|Array|Length _outactors))
  (bind _outactors_2 (Actor|GetAllActorsOfClass "/Script/PainterBall.PurifierTarget"))
  (Variables|Default|SetTotalPurifiersCount (Utilities|Array|Length _outactors_2)))

(event EventOnWin
  (bind _returnvalue (Game|GetPlayerController 0))
  (bind _returnvalue_2 (UserInterface|CreateWidget "/Game/Widgets/WB_Win.WB_Win_C" _returnvalue))
  (UserInterface|Viewport|AddtoViewport _returnvalue_2 0)
  (Input|SetInputModeUIOnly _returnvalue 0 "DoNotLock" false))

(event EventTick
  (params (DeltaSeconds :type Float%20%28single-precision%29)))

(fn ConstructionScript)