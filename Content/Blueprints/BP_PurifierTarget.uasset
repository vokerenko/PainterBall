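; BP_PurifierTarget is a purifier target that toggles its look and plays a sound when a BP_Ball hits it.
; OnChangeColor creates a dynamic material on the mesh, then a FlipFlop alternately plays and reverses a Timeline that blends its roughness and shiny opacity.
; The box overlap plays a random collision sound, with volume scaled by the ball's horizontal speed.
; Nothing in this graph calls OnChangeColor or implements the healing mentioned in its comment.
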(event OnComponentBeginOverlap(Box)
  (params (OverlappedComponent :type Primitive%20Component%20Object%20Reference) (OtherActor :type Actor%20Object%20Reference) (OtherComp :type Primitive%20Component%20Object%20Reference) (OtherBodyIndex :type Integer) (bFromSweep :type Boolean) (SweepResult :type Hit%20Result%20Structure%20%28by%20ref%29))
  (bind _collision_sounds (Variables|Default|GetCollision%20Sounds))
  (bind _asbp_ball (Utilities|Casting|CastToBP_Ball OtherActor))
  (Audio|PlaySound2D (Utilities|Array|Get(acopy) _collision_sounds (Math|Random|RandomIntegerinRange 0 (- (Utilities|Array|Length _collision_sounds) 1))) (/ (+ (Math|Float|Absolute(Float) (.x (Transformation|GetComponentVelocity (Variables|/Script/PainterBall.Ball|GetStaticMesh _asbp_ball)))) (Math|Float|Absolute(Float) (.y (Transformation|GetComponentVelocity (Variables|/Script/PainterBall.Ball|GetStaticMesh _asbp_ball))))) 2e+03) 1.0 0.0 0 0))

(event EventOnChangeColor
  ;[1 1 1] When marked purifier meets another unmarked puriefier the first purifier is healed
  (bind _returnvalue (Rendering|Material|CreateDynamicMaterialInstance (Variables|Default|GetStaticMesh) 0 "/Game/Materials/M_PurifierTargetToBall.M_PurifierTargetToBall" "None" :!class /Script/Engine.PrimitiveComponent))
  (bind _output_get (Variables|Default|SetDMI _returnvalue))
  (Utilities|FlowControl|FlipFlop
    (:A
      (bind _newtrack_2 (Timeline|Timeline PlayFromStart)
        (:Update
          (Rendering|Material|SetScalarParameterValue _output_get "Roughness" (Math|Float|Lerp 0.0 1.0 _newtrack_2) :!class /Script/Engine.MaterialInstanceDynamic)
          (Rendering|Material|SetScalarParameterValue _output_get "Shiny Opacity" (Math|Float|Lerp 7.0 0.0 _newtrack_2) :!class /Script/Engine.MaterialInstanceDynamic))))
    (:B
      (Timeline|Timeline ReverseFromEnd))))

(fn ConstructionScript)